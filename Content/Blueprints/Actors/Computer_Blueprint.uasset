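; Interactable computer actor that opens a quiz menu when the player interacts with it.
; A box overlap registers it as the MainPawn's InteractionActor if none is set and shows its widget, clearing both on exit.
; BeginPlay binds an event to the SelectObject widget's selection.
; InteractwithActor creates the QuizMenu from its answer structure and next level, adds it to the viewport and plays a sound.
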(event OnComponentBeginOverlap(Box)
  (params (OverlappedComponent :type Primitive%20Component%20Object%20Reference) (OtherActor :type Actor%20Object%20Reference) (OtherComp :type Primitive%20Component%20Object%20Reference) (OtherBodyIndex :type Integer) (bFromSweep :type Boolean) (SweepResult :type Hit%20Result%20Structure%20%28by%20ref%29))
  (bind _asmain_pawn (Utilities|Casting|CastToMainPawn OtherActor))
  (Variables|Default|SetAs%20Main%20Pawn _asmain_pawn)
  (Utilities|IsValid (Variables|/Game/Blueprints/Pawns/MainPawn.MainPawn_C|GetInteractionActor _asmain_pawn)
    (:Is%20Not%20Valid
      (Variables|/Game/Blueprints/Pawns/MainPawn.MainPawn_C|SetInteractionActor _asmain_pawn self)
      (CallFunction|ShowWidget true))))

(event OnComponentEndOverlap(Box)
  (params (OverlappedComponent :type Primitive%20Component%20Object%20Reference) (OtherActor :type Actor%20Object%20Reference) (OtherComp :type Primitive%20Component%20Object%20Reference) (OtherBodyIndex :type Integer))
  (bind _asmain_pawn (Utilities|Casting|CastToMainPawn OtherActor))
  (Variables|Default|SetAs%20Main%20Pawn 0)
  (Variables|/Game/Blueprints/Pawns/MainPawn.MainPawn_C|SetInteractionActor _asmain_pawn 0)
  (CallFunction|ShowWidget false))

(event EventInteractwithActor
  (params (Arm? :type Boolean))
  (Utilities|IsValid (Variables|Default|GetQuizMenu)
    (:Is%20Valid
      (Variables|Default|SetQuizMenu 0))
    (:Is%20Not%20Valid
      _))
  (bind _returnvalue (UserInterface|CreateWidget "/Game/Blueprints/Widgets/QuizMenu.QuizMenu_C" 0 (Variables|Default|GetAnswerStructure) (Variables|Default|GetNext%20Level)))
  (bind _output_get (Variables|Default|SetQuizMenu _returnvalue))
  (UserInterface|Viewport|AddtoViewport _output_get 0)
  (Audio|PlaySound2D "/Engine/VREditor/Sounds/UI/Dockable_Window_Drop.Dockable_Window_Drop" 1.0 1.0 0.0 0 0))

(event EventBeginPlay
  (bind _asselect_object (Utilities|Casting|CastToSelectObject (UserInterface|GetUserWidgetObject (Variables|Default|GetWidget))))
  (EventDispatchers|BindEventtoSelected _asselect_object (EventDispatchers|CreateEvent :!event InteractwithActor)))

(fn ConstructionScript)

(fn GetStructure
  (return 0 0 0))

(fn ShowWidget
  (params (bNewVisibility :type Boolean))
  (Rendering|SetVisibility (Variables|Default|GetWidget) bNewVisibility false)
  (return))