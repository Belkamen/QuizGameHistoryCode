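; Interactable lever-like arm actor that swings once and then notifies a linked InteractActor.
; A box overlap registers it as the MainPawn's InteractionActor, if none is set, and shows its widget, whose selection event is bound at BeginPlay.
; Interaction plays a timeline that pitches Arm02 over, then destroys the widget and box, making it single-use, and sends InteractWithActorMessage to the target.
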(event OnComponentBeginOverlap(Box)
  (params (OverlappedComponent :type Primitive%20Component%20Object%20Reference) (OtherActor :type Actor%20Object%20Reference) (OtherComp :type Primitive%20Component%20Object%20Reference) (OtherBodyIndex :type Integer) (bFromSweep :type Boolean) (SweepResult :type Hit%20Result%20Structure%20%28by%20ref%29))
  (bind _asmain_pawn (Utilities|Casting|CastToMainPawn OtherActor))
  (Variables|Default|SetAs%20Main%20Pawn _asmain_pawn)
  (Utilities|IsValid (Variables|/Game/Blueprints/Pawns/MainPawn.MainPawn_C|GetInteractionActor _asmain_pawn)
    (:Is%20Not%20Valid
      (Variables|/Game/Blueprints/Pawns/MainPawn.MainPawn_C|SetInteractionActor _asmain_pawn self)
      (CallFunction|ShowWidget true))))

(event OnComponentEndOverlap(Box)
  (params (OverlappedComponent :type Primitive%20Component%20Object%20Reference) (OtherActor :type Actor%20Object%20Reference) (OtherComp :type Primitive%20Component%20Object%20Reference) (OtherBodyIndex :type Integer))
  (bind _asmain_pawn (Utilities|Casting|CastToMainPawn OtherActor))
  (Variables|Default|SetAs%20Main%20Pawn 0)
  (Variables|/Game/Blueprints/Pawns/MainPawn.MainPawn_C|SetInteractionActor _asmain_pawn 0)
  (CallFunction|ShowWidget false))

(event EventBeginPlay
  (bind _asselect_object (Utilities|Casting|CastToSelectObject (UserInterface|GetUserWidgetObject (Variables|Default|GetWidget))))
  (EventDispatchers|BindEventtoSelected _asselect_object (EventDispatchers|CreateEvent :!event InteractwithActor)))

(event EventInteractwithActor
  (params (Arm? :type Boolean))
  (bind _armalpha (Timeline|ArmLine PlayFromStart)
    (:Update
      (Transformation|SetRelativeRotation (Variables|Default|GetArm_02) (Math|Rotator|MakeRotator 0.0 (Math|Float|Lerp 5e+01 -5e+01 _armalpha) 0.0) false false))
    (:Finished
      (Components|DestroyComponent (Variables|Default|GetWidget))
      (Components|DestroyComponent (Variables|Default|GetBox))
      (Class|InteractionInterface|InteractwithActor(Message) (Variables|Default|GetInteractActor) true))))

(fn ConstructionScript)

(fn ShowWidget
  (params (bNewVisibility :type Boolean))
  (bind _widget (Variables|Default|GetWidget))
  (Utilities|IsValid _widget
    (:Is%20Valid
      (Rendering|SetVisibility _widget bNewVisibility false))
    (:Is%20Not%20Valid
      _))
  (return))