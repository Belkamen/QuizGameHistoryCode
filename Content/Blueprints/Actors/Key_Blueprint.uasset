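; Key pickup actor that gives the player pawn a key identified by KeyID.
; A sphere overlap registers it as the MainPawn's InteractionActor if none is set and shows its widget; leaving clears that reference and hides the widget.
; On BeginPlay it binds an event to the SelectObject widget's selection.
; InteractwithActor calls AddKey on the pawn and, on success, plays a sound and destroys the actor.
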(event OnComponentBeginOverlap(Sphere)
  (params (OverlappedComponent :type Primitive%20Component%20Object%20Reference) (OtherActor :type Actor%20Object%20Reference) (OtherComp :type Primitive%20Component%20Object%20Reference) (OtherBodyIndex :type Integer) (bFromSweep :type Boolean) (SweepResult :type Hit%20Result%20Structure%20%28by%20ref%29))
  (bind _asmain_pawn (Utilities|Casting|CastToMainPawn OtherActor))
  (Variables|Default|SetAs%20Main%20Pawn _asmain_pawn)
  (Utilities|IsValid (Variables|/Game/Blueprints/Pawns/MainPawn.MainPawn_C|GetInteractionActor _asmain_pawn)
    (:Is%20Not%20Valid
      (Variables|/Game/Blueprints/Pawns/MainPawn.MainPawn_C|SetInteractionActor _asmain_pawn self)
      (CallFunction|ShowWidget true))))

(event OnComponentEndOverlap(Sphere)
  (params (OverlappedComponent :type Primitive%20Component%20Object%20Reference) (OtherActor :type Actor%20Object%20Reference) (OtherComp :type Primitive%20Component%20Object%20Reference) (OtherBodyIndex :type Integer))
  (bind _asmain_pawn (Utilities|Casting|CastToMainPawn OtherActor))
  (Variables|Default|SetAs%20Main%20Pawn 0)
  (Variables|/Game/Blueprints/Pawns/MainPawn.MainPawn_C|SetInteractionActor _asmain_pawn 0)
  (CallFunction|ShowWidget false))

(event EventBeginPlay
  (bind _asselect_object (Utilities|Casting|CastToSelectObject (UserInterface|GetUserWidgetObject (Variables|Default|GetWidget))))
  (EventDispatchers|BindEventtoSelected _asselect_object (EventDispatchers|CreateEvent :!event InteractwithActor)))

(event EventInteractwithActor
  (params (Arm? :type Boolean))
  (bind _returnvalue (Default|AddKey (Variables|Default|GetAs%20Main%20Pawn) (Variables|Default|GetKey%20ID)))
  (if _returnvalue
    (Audio|PlaySound2D "/Engine/VREditor/Sounds/UI/Camera_Shutter.Camera_Shutter" 1.0 1.0 0.0 0 0)
    (Actor|DestroyActor)))

(fn ConstructionScript)

(fn ShowWidget
  (params (bNewVisibility :type Boolean))
  (Rendering|SetVisibility (Variables|Default|GetWidget) bNewVisibility false)
  (return))