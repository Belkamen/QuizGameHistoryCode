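; Locked door actor that the player opens with a matching key, or without one when the Arm flag is set.
; A box trigger shows a prompt widget and registers the door as the MainPawn's InteractionActor.
; Interaction, also bound to the widget's selection event, runs chained timelines: the lock rotates and drops with physics, then the door swings by the Inside flag.
; Opening clears the interaction and destroys the trigger; a missing key prints a warning.
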(event OnComponentBeginOverlap(Box)
  (params (OverlappedComponent :type Primitive%20Component%20Object%20Reference) (OtherActor :type Actor%20Object%20Reference) (OtherComp :type Primitive%20Component%20Object%20Reference) (OtherBodyIndex :type Integer) (bFromSweep :type Boolean) (SweepResult :type Hit%20Result%20Structure%20%28by%20ref%29))
  (if (not (Variables|Default|GetbOpen?))
    (CallFunction|ShowWidget true)
    (bind _asmain_pawn (Utilities|Casting|CastToMainPawn OtherActor))
    (Variables|Default|SetAs%20Main%20Pawn _asmain_pawn)
    (Utilities|IsValid (Variables|/Game/Blueprints/Pawns/MainPawn.MainPawn_C|GetInteractionActor _asmain_pawn)
      (:Is%20Not%20Valid
        (Variables|/Game/Blueprints/Pawns/MainPawn.MainPawn_C|SetInteractionActor _asmain_pawn self)))))

(event OnComponentEndOverlap(Box)
  (params (OverlappedComponent :type Primitive%20Component%20Object%20Reference) (OtherActor :type Actor%20Object%20Reference) (OtherComp :type Primitive%20Component%20Object%20Reference) (OtherBodyIndex :type Integer))
  (CallFunction|ShowWidget false)
  (bind _asmain_pawn (Utilities|Casting|CastToMainPawn OtherActor))
  (Variables|Default|SetAs%20Main%20Pawn 0)
  (Variables|/Game/Blueprints/Pawns/MainPawn.MainPawn_C|SetInteractionActor _asmain_pawn 0))

(event Custom|Interact
  (params (Arm? :type Boolean))
  (if (Default|SearchKey (Variables|Default|GetAs%20Main%20Pawn) (Variables|Default|GetKeyIndex))
    (Audio|PlaySound2D "/Game/Assets/SFX/UIMisc_Feedback_36_up_CB_Sounddesign_ACTIVATION2.UIMisc_Feedback_36_up_CB_Sounddesign_ACTIVATION2" 1.0 1.0 0.0 0 0)
    (bind _alphaol (Timeline|AlphaOpenLock PlayFromStart)
      (:Update
        (Transformation|SetRelativeRotation (Variables|Default|GetRotation) (Math|Rotator|MakeRotator (Math|Float|Lerp 0.0 7e+01 _alphaol) 0.0 0.0) false false))
      (:Finished
        (Physics|SetSimulatePhysics (Variables|Default|GetMain) true)
        (Collision|SetCollisionEnabled (Variables|Default|GetStaticMesh) "NoCollision")
        (CallFunction|OpenDoor)))
    (else
      (Development|PrintString "NeedKey!!!" true true "(R=1.000000,G=0.000000,B=0.000000,A=1.000000)"))))

(event Custom|OpenDoor
  (Audio|PlaySound2D "/Game/Assets/SFX/DOORCreak_Wooden_Door__Opening_and_Closing_09_RogueWaves_CreakingDoor__mp3cut_net_.DOORCreak_Wooden_Door__Opening_and_Closing_09_RogueWaves_CreakingDoor__mp3cut_net_" 1.0 1.0 0.0 0 0)
  (bind _alphaod (Timeline|DoorOpen PlayFromStart)
    (:Update
      (Transformation|SetRelativeRotation (Variables|Default|GetStaticMesh) (Math|Rotator|MakeRotator 0.0 0.0 (Math|Float|Lerp 0.0 (Math|Float|SelectFloat -1.6e+02 1.6e+02 (Variables|Default|GetbInside?)) _alphaod)) false false))
    (:Finished
      (Utilities|IsValid (Variables|Default|GetAs%20Main%20Pawn)
        (:Is%20Valid
          (Variables|/Game/Blueprints/Pawns/MainPawn.MainPawn_C|SetInteractionActor (Variables|Default|GetAs%20Main%20Pawn) 0))
        (:Is%20Not%20Valid
          _))
      (Variables|Default|SetAs%20Main%20Pawn 0)
      (Input|DisableInput (Game|GetPlayerController 0))
      (Components|DestroyComponent (Variables|Default|GetBox)))))

(event EventBeginPlay
  (bind _asselect_object (Utilities|Casting|CastToSelectObject (UserInterface|GetUserWidgetObject (Variables|Default|GetWidget))))
  (EventDispatchers|BindEventtoSelected _asselect_object (delegate Custom|Interact)))

(event EventInteractwithActor
  (params (Arm? :type Boolean))
  (if Arm?
    (Audio|PlaySound2D "/Game/Assets/SFX/UIMisc_Feedback_36_up_CB_Sounddesign_ACTIVATION2.UIMisc_Feedback_36_up_CB_Sounddesign_ACTIVATION2" 1.0 1.0 0.0 0 0 :!label _label)
    (bind _alphaol (Timeline|AlphaOpenLock PlayFromStart)
      (:Update
        (Transformation|SetRelativeRotation (Variables|Default|GetRotation) (Math|Rotator|MakeRotator (Math|Float|Lerp 0.0 7e+01 _alphaol) 0.0 0.0) false false))
      (:Finished
        (Physics|SetSimulatePhysics (Variables|Default|GetMain) true)
        (Collision|SetCollisionEnabled (Variables|Default|GetStaticMesh) "NoCollision")
        (CallFunction|OpenDoor)))
    (elif (Default|SearchKey (Variables|Default|GetAs%20Main%20Pawn) (Variables|Default|GetKeyIndex))
      (goto _label)
      (else
        (Development|PrintString "NeedKey!!!" true true "(R=1.000000,G=0.000000,B=0.000000,A=1.000000)")))))

(fn ConstructionScript)

(fn ShowWidget
  (params (bNewVisibility :type Boolean))
  (Rendering|SetVisibility (Variables|Default|GetWidget) bNewVisibility false)
  (return))