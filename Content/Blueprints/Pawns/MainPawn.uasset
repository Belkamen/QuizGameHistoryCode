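; MainPawn is a player pawn with click-to-move control and a collection of key IDs.
; Right-click traces under the cursor, replaces the Target_MouseLocation marker slightly above the hit, then calls Follow for one movement input and SimpleMoveToLocation for navigation.
; SearchKey and AddKey check and uniquely add IDs in KeyIDs.
; An InteractionActor message call exists but is unwired, so it never runs.
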(event Input|KeyboardEvents|E
  (params (Key :type Key%20Structure :default "None")))

(event Input|MouseEvents|RightMouseButton
  (params (Key :type Key%20Structure :default "None"))
  (bind _returnvalue (Game|GetPlayerController 0))
  (bind _array (Utilities|Array|MakeArray "ObjectTypeQuery7"))
  (bind _hitresult (Class|PlayerController|GetHitResultUnderCursorforObjects _returnvalue _array true))
  (bind _location (Collision|BreakHitResult _hitresult))
  (bind _returnvalue_2 (+ _location "0.000000,0.000000,35.000000"))
  (:Pressed
    (Utilities|IsValid (Variables|Default|GetMouseTarget)
      (:Is%20Valid
        (Actor|DestroyActor (Variables|Default|GetMouseTarget)))
      (:Is%20Not%20Valid
        _))
    (bind _returnvalue_3 (Game|SpawnActorfromClass "/Game/Blueprints/Actors/Mouse/Target_MouseLocation.Target_MouseLocation_C" (Math|Transform|MakeTransform _returnvalue_2 "0, 0, 0" "1.000000,1.000000,1.000000") "AlwaysSpawn" "MultiplyWithRoot" self 0))
    (Variables|Default|SetMouseTarget _returnvalue_3)
    (CallFunction|Follow _returnvalue_2)
    (AI|Navigation|SimpleMovetoLocation (Game|GetPlayerController 0) _returnvalue_2)))

(fn ConstructionScript)

(fn SearchKey
  (params (ItemToFind :type Integer%20%28by%20ref%29))
  (return (Utilities|Array|ContainsItem (Variables|Default|GetKeyIDs) ItemToFind)))

(fn AddKey
  (params (KeyID :type Integer%20%28by%20ref%29))
  (bind _keyids (Variables|Default|GetKeyIDs))
  (bind _returnvalue (Utilities|Array|AddUnique _keyids KeyID))
  (return (== KeyID (Utilities|Array|Get(acopy) _keyids _returnvalue))))

(fn Follow
  (params (Location :type Vector))
  (Pawn|Input|AddMovementInput (Math|Vector|GetUnitDirection(Vector) (Transformation|GetActorLocation) Location) 1.0 false))